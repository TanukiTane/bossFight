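; Enemy bullet actor with a projectile movement component that can be turned into a homing missile.
; The AutoBullet event adds a new child actor component to the given target and uses it as the homing target.
; If that component is valid, it enables homing with a set acceleration and gives the bullet a short lifespan.
; The graph has no active overlap, damage or tick logic.
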(event `AutoBullet`
  (params (Target :type "/Game/ThirdPerson/Blueprints/BP_ThirdPersonCharacter Object Reference"))
  (bind _projectilemovement (`self.ProjectileMovement`))
  ;[1 1 1] Messile
  (bind _returnvalue (`AddComponent|NODE_AddChildActorComponent-0` :`self` Target))
  (if (`KismetSystemLibrary.IsValid` _returnvalue)
    (set `ProjectileMovementComponent.HomingTargetComponent` _returnvalue _projectilemovement)
    (set `ProjectileMovementComponent.bIsHomingProjectile` true _projectilemovement)
    (set `ProjectileMovementComponent.HomingAccelerationMagnitude` 5000.0 _projectilemovement)
    (`self.SetLifeSpan` 2.0)))

(fn `UserConstructionScript`
  (`parent.UserConstructionScript`))