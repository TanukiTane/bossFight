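; BP_bullet is a projectile actor that damages the player or enemies it hits.
; Its Box component's hit event casts the other actor to BP_ThirdPersonCharacter and BP_enemy in sequence, applying point damage from the Damage variable to whichever matches.
; The bullet credits its instigator's controller as the damage instigator and destroys itself after any hit, whether or not a cast succeeds.
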(event `self.Box.OnComponentHit`
  (params (HitComponent :type "PrimitiveComponent Object Reference") (OtherActor :type "Actor Object Reference") (OtherComp :type "PrimitiveComponent Object Reference") (NormalImpulse :type "Vector Structure") (Hit :type "HitResult Structure (by ref)"))
  (`|ExecutionSequence`
    (:`then_0`
      ;[1 1 1] Player Damage
      (bind _asbp_third_person_character (cast `/Game/ThirdPerson/Blueprints/BP_ThirdPersonCharacter` OtherActor))
      (bind _output_get (set `self.Character` _asbp_third_person_character))
      (`GameplayStatics.ApplyPointDamage` _output_get (`self.Damage`) NormalImpulse Hit (`self.GetInstigatorController`) self))
    (:`then_1`
      ;[1 1 1] Enemy Damage
      (bind _asbp_enemy (cast `/Game/Enemy/BP_enemy` OtherActor))
      (bind _output_get_2 (set `self.Enemy` _asbp_enemy))
      (`GameplayStatics.ApplyPointDamage` _output_get_2 (`self.Damage`) NormalImpulse Hit (`self.GetInstigatorController`) self))
    (:`then_2`
      (`self.K2_DestroyActor`))))

(fn `UserConstructionScript`)