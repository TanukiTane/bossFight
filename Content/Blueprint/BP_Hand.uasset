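; BP_Hand is a projectile hand, apparently an enemy attack, that stops on its first bounce and exposes three shootable weak spots.
; A direct hit on BP_ThirdPersonCharacter destroys it, while other impacts reveal the spots and apply radial falloff damage that ignores the Enemy.
; Each spot sphere counts down its own lives under BP_bullet hits, then hides and disables collision.
; The hand destroys itself when the shared spot count reaches zero.
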(event `self.ReceiveBeginPlay`)

(event `self.Cylinder.OnComponentHit`
  (params (HitComponent :type "PrimitiveComponent Object Reference") (OtherActor :type "Actor Object Reference") (OtherComp :type "PrimitiveComponent Object Reference") (NormalImpulse :type "Vector Structure") (Hit :type "HitResult Structure (by ref)"))
  (bind (_bblockinghit _binitialoverlap _time _distance _location _impactpoint _normal _impactnormal _physmat _hitactor) (`GameplayStatics.BreakHitResult` Hit))
  ;[1 1 1] Radial Damage
  (bind _asbp_third_person_character (cast `/Game/ThirdPerson/Blueprints/BP_ThirdPersonCharacter` _hitactor)
    (:`then`
      (set `self.Character` _asbp_third_person_character)
      (`self.K2_DestroyActor`)
      (goto _label :!via `Reset`))
    (:`CastFailed`
      (`self.ShowSpots`)
      (`GameplayStatics.ApplyRadialDamageWithFalloff` 25.0 5.0 _location 500.0 2500.0 5.0 null (`|MakeArray` (`self.Enemy`) self :!type "Actor Object Reference") null null)
      (`/Engine/EditorBlueprintResources/StandardMacros.DoOnce` false :!label _label))))

(event `self.Sphere.OnComponentHit`
  (params (HitComponent :type "PrimitiveComponent Object Reference") (OtherActor :type "Actor Object Reference") (OtherComp :type "PrimitiveComponent Object Reference") (NormalImpulse :type "Vector Structure") (Hit :type "HitResult Structure (by ref)"))
  (bind _sphere (`self.Sphere`))
  ;[1 1 1] kill spot logic
  (cast `/Game/Blueprint/BP_bullet` OtherActor)
  (if (== (`self.Live`) 0)
    (`SceneComponent.SetHiddenInGame` _sphere true false)
    (`PrimitiveComponent.SetCollisionEnabled` _sphere "NoCollision")
    (bind _result (`/Engine/EditorBlueprintResources/StandardMacros.DecrementInt` (`self.NumberOfSpots`) :!label _label_2)
      (:`  `
        (bind _output_get (set `self.NumberOfSpots` _result))
        (if (== _output_get 0)
          (`self.K2_DestroyActor`))))
    (else
      (`/Engine/EditorBlueprintResources/StandardMacros.DecrementInt` (`self.Live`)))))

(event `self.Sphere1.OnComponentHit`
  (params (HitComponent :type "PrimitiveComponent Object Reference") (OtherActor :type "Actor Object Reference") (OtherComp :type "PrimitiveComponent Object Reference") (NormalImpulse :type "Vector Structure") (Hit :type "HitResult Structure (by ref)"))
  (bind _sphere1 (`self.Sphere1`))
  ;[1 1 1] kill spot logic
  (cast `/Game/Blueprint/BP_bullet` OtherActor)
  (if (== (`self.Live1`) 0)
    (`SceneComponent.SetHiddenInGame` _sphere1 true false)
    (`PrimitiveComponent.SetCollisionEnabled` _sphere1 "NoCollision")
    (goto _label_2)
    (else
      (`/Engine/EditorBlueprintResources/StandardMacros.DecrementInt` (`self.Live1`)))))

(event `self.Sphere2.OnComponentHit`
  (params (HitComponent :type "PrimitiveComponent Object Reference") (OtherActor :type "Actor Object Reference") (OtherComp :type "PrimitiveComponent Object Reference") (NormalImpulse :type "Vector Structure") (Hit :type "HitResult Structure (by ref)"))
  (bind _sphere2 (`self.Sphere2`))
  ;[1 1 1] kill spot logic
  (cast `/Game/Blueprint/BP_bullet` OtherActor)
  (if (== (`self.Live2`) 0)
    (`SceneComponent.SetHiddenInGame` _sphere2 true false)
    (`PrimitiveComponent.SetCollisionEnabled` _sphere2 "NoCollision")
    (goto _label_2)
    (else
      (`/Engine/EditorBlueprintResources/StandardMacros.DecrementInt` (`self.Live2`)))))

(event `self.ProjectileMovement.OnProjectileBounce`
  (params (ImpactResult :type "HitResult Structure (by ref)") (ImpactVelocity :type "Vector Structure (by ref)"))
  ;[1 1 1] Stop Movement on Floor
  (`MovementComponent.StopMovementImmediately` (`self.ProjectileMovement`)))

(fn `ShowSpots`
  (bind _sphere (`self.Sphere`))
  (bind _cylinder (`self.Cylinder`))
  (`SceneComponent.SetVisibility` _sphere true false)
  (`SceneComponent.SetVisibility` (`self.Sphere1`) true false)
  (`SceneComponent.SetVisibility` (`self.Sphere2`) true false)
  (`|ExecutionSequence`
    (:`then_0`
      (`SceneComponent.K2_AttachToComponent` _sphere _cylinder "Weak1" "KeepWorld" "KeepWorld" "KeepWorld" true))
    (:`then_1`
      (`SceneComponent.K2_AttachToComponent` (`self.Sphere1`) _cylinder "Weak2" "KeepWorld" "KeepWorld" "KeepWorld" true))
    (:`then_2`
      (`SceneComponent.K2_AttachToComponent` (`self.Sphere2`) _cylinder "Weak1" "KeepWorld" "KeepWorld" "KeepWorld" true))))

(fn `UserConstructionScript`)