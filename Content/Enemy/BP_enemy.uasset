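; Enemy that fires BP_EnemyBullet at a sensed third-person player and periodically drops a hand attack above them.
; PawnSensing starts a looping Fire timer, which yaws the enemy toward the player and launches bullets at that target.
; After several sightings, counted in Shoots, it spawns BP_Hand and pauses shooting; StartHit resumes fire once the hand is gone.
; Point damage only prints a debug message.
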(event `self.ReceiveTick`
  (params (DeltaSeconds :type "Float (single-precision)")))

(event `self.PawnSensing.OnSeePawn`
  (params (Pawn :type "Pawn Object Reference"))
  (bind _asbp_third_person_character (cast `/Game/ThirdPerson/Blueprints/BP_ThirdPersonCharacter` Pawn))
  (set `self.GoalPlayer` _asbp_third_person_character)
  (`self.Fire`)
  (bind _returnvalue (`KismetSystemLibrary.K2_SetTimer` null "Fire" 0.5 true))
  (set `self.TimerFire` _returnvalue)
  (bind _result (`/Engine/EditorBlueprintResources/StandardMacros.IncrementInt` (`self.Shoots`))
    (:`  `
      (bind _output_get (set `self.Shoots` _result))
      (if (> _output_get 5)
        (`self.SpawnHand`)
        (set `self.Stop` true)))))

(event `self.ReceivePointDamage`
  (params (Damage :type "Float (single-precision)") (DamageType :type "DamageType Object Reference") (HitLocation :type "Vector Structure") (HitNormal :type "Vector Structure") (HitComponent :type "PrimitiveComponent Object Reference") (BoneName :type Name) (ShotFromDirection :type "Vector Structure") (InstigatedBy :type "Controller Object Reference") (DamageCauser :type "Actor Object Reference") (HitInfo :type "HitResult Structure (by ref)"))
  (`KismetSystemLibrary.PrintString` "TakeDamage"))

(fn `Fire`
  (`self.TurnToGoal`)
  (if (`self.Stop`)
    (`KismetSystemLibrary.K2_SetTimer` null "StartHit" 3.0 true)
    (`self.StartHit`)
    (else
      (bind _returnvalue (`|SpawnActorFromClass` "/Game/Blueprint/BP_EnemyBullet.BP_EnemyBullet_C" (`KismetMathLibrary.MakeTransform` (`SceneComponent.K2_GetComponentLocation` (`self.BulletSpawnLocation`)) (`self.Rotator`)) "AlwaysSpawn" "MultiplyWithRoot" self (`self.GetInstigator`)))
      (`/Game/Blueprint/BP_EnemyBullet.AutoBullet` _returnvalue (`self.GoalPlayer`)))))

(fn `SpawnHand`
  (bind (_returnvalue_x _returnvalue_y _returnvalue_z) (`KismetMathLibrary.BreakVector` (`self.K2_GetActorLocation` (`self.GoalPlayer`))))
  (if (not (`self.Stop`))
    (bind _returnvalue (`|SpawnActorFromClass` "/Game/Blueprint/BP_Hand.BP_Hand_C" (`KismetMathLibrary.MakeTransform` (`KismetMathLibrary.MakeVector` _returnvalue_x _returnvalue_y (+ _returnvalue_z 250.0))) "AlwaysSpawn" "MultiplyWithRoot" null null))
    (set `self.Hand` _returnvalue)))

(fn `StartHit`
  (if (not (`KismetSystemLibrary.IsValid` (`self.Hand`)))
    (set `self.Stop` false)
    (set `self.Shoots` 0)
    (set `self.Hand` null)))

(fn `TurnToGoal`
  (bind (_returnvalue_roll _returnvalue_pitch) (`KismetMathLibrary.BreakRotator` (`self.K2_GetActorRotation` self)))
  (bind _goalplayer (`self.GoalPlayer`)
    (:`then`
      (bind _output_get (set `self.Rotator` (`KismetMathLibrary.MakeRotator` _returnvalue_roll _returnvalue_pitch (.yaw (`KismetMathLibrary.FindLookAtRotation` (`self.K2_GetActorLocation` self) (`self.K2_GetActorLocation` _goalplayer))))))
      (`self.K2_SetActorRotation` self _output_get false)
      (set `self.LocationGoal` (`self.K2_GetActorLocation` _goalplayer))
      (return))
    (:`else`)))

(fn `UserConstructionScript`)